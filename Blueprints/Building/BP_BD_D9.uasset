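; Building actor for D9 that toggles day/night materials and highlights a selected floor on its static mesh.
; The 材质切换 event uses a FlipFlop to alternate night and default glass and wall materials.
; 选中楼层 caches the material at Index and applies CubeMaterial; 取消选中楼层 restores it if IsSelected.
; Selection has no guard, so repeated selection overwrites the cached original.
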(event EventBeginPlay)

(event Collision|EventActorBeginOverlap
  (params (OtherActor :type Actor%20Object%20Reference)))

(event EventTick
  (params (DeltaSeconds :type Float%20%28single-precision%29)))

(event Event选中楼层
  (bind _staticmesh_0 (Variables|Default|GetStaticMesh_0))
  (bind _index (Variables|Default|Getindex))
  (Variables|Default|SetoldMertrial (Rendering|Material|GetMaterial _staticmesh_0 _index))
  (Rendering|Material|SetMaterial _staticmesh_0 _index "/Game/Common/Materials/CubeMaterial.CubeMaterial")
  (Variables|Default|SetisSelected true))

(event Event取消选中楼层
  (if (Variables|Default|GetisSelected)
    (Rendering|Material|SetMaterial (Variables|Default|GetStaticMesh_0) (Variables|Default|Getindex) (Variables|Default|GetoldMertrial))
    (Variables|Default|SetisSelected false)))

(event Event材质切换
  (bind _staticmesh_0 (Variables|Default|GetStaticMesh_0))
  (Utilities|FlowControl|FlipFlop
    (:A
      (Rendering|Material|SetMaterial _staticmesh_0 0 "/Game/Common/Materials/Buildings/M_Night_Glass.M_Night_Glass")
      (Rendering|Material|SetMaterial _staticmesh_0 1 "/Game/Common/Materials/Buildings/M_Night_Wall1.M_Night_Wall1"))
    (:B
      (Rendering|Material|SetMaterial _staticmesh_0 0 "/Game/Common/Materials/Buildings/M_Glass.M_Glass")
      (Rendering|Material|SetMaterial _staticmesh_0 1 "/Game/Common/Materials/Buildings/M_Wall.M_Wall"))))

(fn ConstructionScript)