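; Day/night switcher actor that toggles the level between bright day and dim night presets, starting in day on BeginPlay.
; It creates a hidden slider widget and binds its dispatchers to handlers for directional light intensity and pitch, skylight intensity, and sky sphere clouds.
; The 时间切换 event uses a FlipFlop to push each preset through those dispatchers, so the widget acts as the relay to the scene.
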(event Custom|自定义事件_0
  (params (Skylight :type Float%20%28single-precision%29))
  ;[1 1 1] 天空光源强度
  (Rendering|Components|Light|SetIntensity (Variables|/Script/Engine.SkyLight|GetLightComponent (Variables|Default|GetSkyLight)) Skylight))

(event Custom|光源强度
  (params (Light :type Float%20%28single-precision%29))
  ;[1 1 1] 定向光源强度
  (Rendering|Components|Light|SetIntensity (Variables|/Script/Engine.Light|GetLightComponent (Variables|Default|GetLight)) Light))

(event Custom|时间切换
  (bind _bp_ui_daylight_sider (Variables|Default|GetBp_UI_DayLight_Sider))
  (Utilities|FlowControl|FlipFlop
    (:A
      (Default|CallSunHeight _bp_ui_daylight_sider -85.0)
      (Default|CallLight _bp_ui_daylight_sider 3.6)
      (Default|CallSkylight _bp_ui_daylight_sider 1.0)
      (Default|CallCloudOpacity _bp_ui_daylight_sider 1.0))
    (:B
      (Default|CallSunHeight _bp_ui_daylight_sider 85.0)
      (Default|CallLight _bp_ui_daylight_sider 0.1)
      (Default|CallSkylight _bp_ui_daylight_sider 0.5)
      (Default|CallCloudOpacity _bp_ui_daylight_sider 0.1))))

(event Custom|定向光源高度
  (params (SunHeight :type Float%20%28single-precision%29))
  ;[1 1 1] 太阳高度
  (Transformation|SetRelativeRotation (Variables|/Script/Engine.Actor|GetRootComponent (Variables|Default|GetLight)) (Math|Rotator|MakeRotator 0.0 (+ SunHeight (Variables|Default|GetsunSpeed)) 0.0) false false)
  (Default|UpdateSunDirection (Variables|Default|GetBP_sky_Sphere)))

(event Custom|init
  (bind _bp_ui_daylight_sider (Variables|Default|GetBp_UI_DayLight_Sider))
  (Utilities|FlowControl|FlipFlop
    (:A
      (Default|CallSunHeight _bp_ui_daylight_sider -85.0)
      (Default|CallLight _bp_ui_daylight_sider 3.6)
      (Default|CallSkylight _bp_ui_daylight_sider 1.0)
      (Default|CallCloudOpacity _bp_ui_daylight_sider 1.0))
    (:B
      (Default|CallSunHeight _bp_ui_daylight_sider 85.0)
      (Default|CallLight _bp_ui_daylight_sider 0.1)
      (Default|CallSkylight _bp_ui_daylight_sider 0.5)
      (Default|CallCloudOpacity _bp_ui_daylight_sider 0.1))))

(event Custom|天空球云透明度
  (params (CloudOpacity :type Float%20%28single-precision%29))
  ;[1 1 1] 天空球云透明度
  (Default|ChangeClould (Variables|Default|GetBP_sky_Sphere) CloudOpacity))

(event EventBeginPlay
  (bind _returnvalue (Game|GetPlayerController 0))
  ;[1 1 1] 创建视口UI
  (bind _returnvalue_2 (UserInterface|CreateWidget "/Game/common/Blueprints/Materials/Bp_UI_DayLight_Sider.Bp_UI_DayLight_Sider_C"))
  (bind _output_get (Variables|Default|SetBp_UI_DayLight_Sider _returnvalue_2))
  (UserInterface|Viewport|AddtoViewport _output_get 0)
  (Input|EnableInput _returnvalue)
  (Variables|/Script/Engine.PlayerController|SetbShowMouseCursor _returnvalue true)
  (Actor|GetActorOfClass "/Engine/EngineSky/BP_Sky_Sphere.BP_Sky_Sphere_C")
  (Utilities|FlowControl|Sequence
    (:then_0
      ;[1 1 1] 定向光源强度
      (EventDispatchers|BindEventtoLight (Variables|Default|GetBp_UI_DayLight_Sider) (delegate Custom|光源强度)))
    (:then_1
      ;[1 1 1] 天空光源强度
      (EventDispatchers|BindEventtoSkylight (Variables|Default|GetBp_UI_DayLight_Sider) (delegate Custom|自定义事件_0)))
    (:then_2
      ;[1 1 1] 天空球云透明度
      (EventDispatchers|BindEventtoCloudOpacity (Variables|Default|GetBp_UI_DayLight_Sider) (delegate Custom|天空球云透明度)))
    (:then_3
      ;[1 1 1] 太阳高度
      (EventDispatchers|BindEventtoSunHeight (Variables|Default|GetBp_UI_DayLight_Sider) (delegate Custom|定向光源高度)))
    (:then_4
      (Widget|SetVisibility (Variables|Default|GetBp_UI_DayLight_Sider) "Hidden"))
    (:then_5
      (CallFunction|Init))))

(fn ConstructionScript
  (Rendering|Material|CreateDynamicMaterialInstance 0 "None" :!class /Script/Engine.KismetMaterialLibrary))