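; Player character for a walkable scene that switches between manual movement and an automatic looping tour along numbered waypoints.
; Custom events pass move and look input through only while the tour is off; the space event toggles it and changes the spring arm's rotation lag.
; During the tour, a listener event steers toward the current point, using a 2D distance check to advance and wrap around.
; Logic for snapping back to the previous point is unconnected.
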(event Custom|CA_空格事件
  (bind _springarm (Variables|Default|GetSpringArm))
  ;[1 1 1] 人物空格事件
  (bind _output_get (Variables|Default|SetIsMoving (not (Variables|Default|GetIsMoving))))
  (if _output_get
    (Variables|/Script/Engine.SpringArmComponent|SetCameraRotationLagSpeed _springarm 2.0)
    (else
      (Variables|/Script/Engine.SpringArmComponent|SetCameraRotationLagSpeed _springarm 4e+01))))

(event Custom|CA_监听走动事件
  ;[1 1 1] 人物走动事件监听
  (if (Variables|Default|GetIsMoving)
    (if (CallFunction|Check)
      (bind _result (Math|Integer|IncrementInt (Variables|Default|GetCurrentPointIndex))
        (:%20%20
          (if (> _result (Variables|Default|GetPointAmount))
            (Variables|Default|SetCurrentPointIndex 1)
            (Variables|Default|Setnotfirstround true))))
      (elif (.ReturnValue (Utilities|Map|Find (Variables|Default|GetPoints) (Variables|Default|GetCurrentPointIndex)))
        (Pawn|Input|AddMovementInput (Math|Vector|Normalize (- (Transformation|GetActorLocation (.Value (Utilities|Map|Find (Variables|Default|GetPoints) (Variables|Default|GetCurrentPointIndex)))) (Transformation|GetActorLocation))) 1.0 false)
        (Pawn|SetControlRotation (Pawn|GetController) (Math|Rotator|MakeRotator 0.0 0.0 (.Yaw (Math|Rotator|BreakRotator (Math|Rotator|MakeRotfromX (Math|Vector|Normalize (- (Transformation|GetActorLocation (.Value (Utilities|Map|Find (Variables|Default|GetPoints) (Variables|Default|GetCurrentPointIndex)))) (Transformation|GetActorLocation))))))))))))

(event Custom|CA_MoveRight
  (params (ScaleValue :type Float%20%28single-precision%29))
  ;[1 1 1] 人物左右移动
  (if (not (Variables|Default|GetIsMoving))
    (Pawn|Input|AddMovementInput (Transformation|GetActorRightVector) ScaleValue false)))

(event Custom|CA_LookUp
  (params (Val :type Float%20%28single-precision%29))
  ;[1 1 1] 人物LookUp
  (if (not (Variables|Default|GetIsMoving))
    (Pawn|Input|AddControllerPitchInput Val)))

(event Custom|CA_Turn
  (params (Val :type Float%20%28single-precision%29))
  ;[1 1 1] 人物Turn
  (if (not (Variables|Default|GetIsMoving))
    (Pawn|Input|AddControllerYawInput Val)))

(event Custom|CA_MoveForward
  (params (ScaleValue :type Float%20%28single-precision%29))
  ;[1 1 1] 人物往前走事件
  (if (not (Variables|Default|GetIsMoving))
    (Pawn|Input|AddMovementInput (Transformation|GetActorForwardVector) ScaleValue false)))

(event EventBeginPlay
  (Variables|/Script/Engine.PlayerController|SetbShowMouseCursor (Game|GetPlayerController 0) true))

(fn ConstructionScript)

(fn Check
  (bind _points (Variables|Default|GetPoints))
  (bind _currentpointindex (Variables|Default|GetCurrentPointIndex))
  (bind (_value _returnvalue) (Utilities|Map|Find _points _currentpointindex))
  (if _returnvalue
    (return (<= (Math|Vector2D|Vector2DLength (- (Math|Conversions|ToVector2D(Vector) (Transformation|GetActorLocation)) (Math|Conversions|ToVector2D(Vector) (Transformation|GetActorLocation _value)))) 5e+01))
    (else
      (return false))))