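; IoT air conditioner actor that shows an on, off or warning state and opens a detail popup when clicked.
; InitItem stores its data, then scales one of three variants visible and selects its label widget, passing temperature to the normal one.
; Tick turns the active label toward the camera and spins the fan while on.
; If operable, clicks blend the view here, replace the popup and flag focus on DCLogic.
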(event OnClicked(Widget)
  (params (TouchedComponent :type Primitive%20Component%20Object%20Reference) (ButtonPressed :type Key%20Structure :default "None"))
  ;[1 1 1] 查看正常状态信息
  (if (Variables|Default|GetoperateState)
    (Game|Player|SetViewTargetwithBlend (Game|GetPlayerController 0) self 0.5 "VTBlend_Linear" 0.0 false)
    (bind _foundwidgets (Widget|GetAllWidgetsOfClass "/Game/Common/Blueprints/IOT/AirConditioner/BP_UI_TanChang_Air-Conditioning_Normal.BP_UI_TanChang_Air-Conditioning_Normal_C" true))
    (for _array_element _foundwidgets
      (Widget|RemovefromParent _array_element))
    (bind _returnvalue (UserInterface|CreateWidget "/Game/Common/Blueprints/IOT/AirConditioner/BP_UI_TanChang_Air-Conditioning_Normal.BP_UI_TanChang_Air-Conditioning_Normal_C"))
    (Default|InitItemData _returnvalue (Variables|Default|Getid) self (Variables|Default|Getremarks))
    (UserInterface|Viewport|AddtoViewport _returnvalue 0)
    (Variables|/Game/Common/Blueprints/Sence/DC/DCLogic.DCLogic_C|SetisFocusAirConditioner (Variables|Default|GetdcLogic) true)))

(event OnClicked(Widget1)
  (params (TouchedComponent :type Primitive%20Component%20Object%20Reference) (ButtonPressed :type Key%20Structure :default "None"))
  ;[1 1 1] 查看关闭状态信息
  (if (Variables|Default|GetoperateState)
    (Game|Player|SetViewTargetwithBlend (Game|GetPlayerController 0) self 0.5 "VTBlend_Linear" 0.0 false)
    (bind _foundwidgets (Widget|GetAllWidgetsOfClass "/Game/Common/Blueprints/IOT/AirConditioner/BP_UI_TanChang_Air-Conditioning_Normal.BP_UI_TanChang_Air-Conditioning_Normal_C" true))
    (for _array_element _foundwidgets
      (Widget|RemovefromParent _array_element))
    (bind _returnvalue (UserInterface|CreateWidget "/Game/Common/Blueprints/IOT/AirConditioner/BP_UI_TanChang_Air-Conditioning_Normal.BP_UI_TanChang_Air-Conditioning_Normal_C"))
    (Default|InitItemData _returnvalue (Variables|Default|Getid) self (Variables|Default|Getremarks))
    (UserInterface|Viewport|AddtoViewport _returnvalue 0)
    (Variables|/Game/Common/Blueprints/Sence/DC/DCLogic.DCLogic_C|SetisFocusAirConditioner (Variables|Default|GetdcLogic) true)))

(event OnClicked(Widget2)
  (params (TouchedComponent :type Primitive%20Component%20Object%20Reference) (ButtonPressed :type Key%20Structure :default "None"))
  ;[1 1 1] 查看错误状态信息
  (if (Variables|Default|GetoperateState)
    (Game|Player|SetViewTargetwithBlend (Game|GetPlayerController 0) self 0.5 "VTBlend_Linear" 0.0 false)
    (bind _foundwidgets (Widget|GetAllWidgetsOfClass "/Game/Common/Blueprints/IOT/AirConditioner/BP_UI_TanChang_Air-Conditioning_Normal.BP_UI_TanChang_Air-Conditioning_Normal_C" true))
    (for _array_element _foundwidgets
      (Widget|RemovefromParent _array_element))
    (bind _returnvalue (UserInterface|CreateWidget "/Game/Common/Blueprints/IOT/AirConditioner/BP_UI_TanChang_Air-Conditioning_Normal.BP_UI_TanChang_Air-Conditioning_Normal_C"))
    (Default|InitItemData _returnvalue (Variables|Default|Getid) self (Variables|Default|Getremarks))
    (UserInterface|Viewport|AddtoViewport _returnvalue 0)
    (Variables|/Game/Common/Blueprints/Sence/DC/DCLogic.DCLogic_C|SetisFocusAirConditioner (Variables|Default|GetdcLogic) true)))

(event OnClicked(SM_FSK)
  (params (TouchedComponent :type Primitive%20Component%20Object%20Reference) (ButtonPressed :type Key%20Structure :default "None"))
  ;[1 1 1] 查看正常状态信息
  (if (Variables|Default|GetoperateState)
    (Game|Player|SetViewTargetwithBlend (Game|GetPlayerController 0) self 0.5 "VTBlend_Linear" 0.0 false)
    (bind _foundwidgets (Widget|GetAllWidgetsOfClass "/Game/Common/Blueprints/IOT/AirConditioner/BP_UI_TanChang_Air-Conditioning_Normal.BP_UI_TanChang_Air-Conditioning_Normal_C" true))
    (for _array_element _foundwidgets
      (Widget|RemovefromParent _array_element))
    (bind _returnvalue (UserInterface|CreateWidget "/Game/Common/Blueprints/IOT/AirConditioner/BP_UI_TanChang_Air-Conditioning_Normal.BP_UI_TanChang_Air-Conditioning_Normal_C"))
    (Default|InitItemData _returnvalue (Variables|Default|Getid) self (Variables|Default|Getremarks))
    (UserInterface|Viewport|AddtoViewport _returnvalue 0)
    (Variables|/Game/Common/Blueprints/Sence/DC/DCLogic.DCLogic_C|SetisFocusAirConditioner (Variables|Default|GetdcLogic) true)))

(event OnClicked(SM_FSK1)
  (params (TouchedComponent :type Primitive%20Component%20Object%20Reference) (ButtonPressed :type Key%20Structure :default "None"))
  ;[1 1 1] 查看关闭状态信息
  (if (Variables|Default|GetoperateState)
    (Game|Player|SetViewTargetwithBlend (Game|GetPlayerController 0) self 0.5 "VTBlend_Linear" 0.0 false)
    (bind _foundwidgets (Widget|GetAllWidgetsOfClass "/Game/Common/Blueprints/IOT/AirConditioner/BP_UI_TanChang_Air-Conditioning_Normal.BP_UI_TanChang_Air-Conditioning_Normal_C" true))
    (for _array_element _foundwidgets
      (Widget|RemovefromParent _array_element))
    (bind _returnvalue (UserInterface|CreateWidget "/Game/Common/Blueprints/IOT/AirConditioner/BP_UI_TanChang_Air-Conditioning_Normal.BP_UI_TanChang_Air-Conditioning_Normal_C"))
    (Default|InitItemData _returnvalue (Variables|Default|Getid) self (Variables|Default|Getremarks))
    (UserInterface|Viewport|AddtoViewport _returnvalue 0)
    (Variables|/Game/Common/Blueprints/Sence/DC/DCLogic.DCLogic_C|SetisFocusAirConditioner (Variables|Default|GetdcLogic) true)))

(event OnClicked(SM_FSK2)
  (params (TouchedComponent :type Primitive%20Component%20Object%20Reference) (ButtonPressed :type Key%20Structure :default "None"))
  ;[1 1 1] 查看错误状态信息
  (if (Variables|Default|GetoperateState)
    (Game|Player|SetViewTargetwithBlend (Game|GetPlayerController 0) self 0.5 "VTBlend_Linear" 0.0 false)
    (bind _foundwidgets (Widget|GetAllWidgetsOfClass "/Game/Common/Blueprints/IOT/AirConditioner/BP_UI_TanChang_Air-Conditioning_Normal.BP_UI_TanChang_Air-Conditioning_Normal_C" true))
    (for _array_element _foundwidgets
      (Widget|RemovefromParent _array_element))
    (bind _returnvalue (UserInterface|CreateWidget "/Game/Common/Blueprints/IOT/AirConditioner/BP_UI_TanChang_Air-Conditioning_Normal.BP_UI_TanChang_Air-Conditioning_Normal_C"))
    (Default|InitItemData _returnvalue (Variables|Default|Getid) self (Variables|Default|Getremarks))
    (UserInterface|Viewport|AddtoViewport _returnvalue 0)
    (Variables|/Game/Common/Blueprints/Sence/DC/DCLogic.DCLogic_C|SetisFocusAirConditioner (Variables|Default|GetdcLogic) true)))

(event Custom|initAirCondition
  (params (state :type String))
  (bind _normal (Variables|Default|GetNormal))
  (bind _close (Variables|Default|GetClose))
  (bind _warning (Variables|Default|GetWarning))
  (bind _widget (Variables|Default|GetWidget))
  ;[1 1 1] 初始化空调状态
  (bind _output_get (Variables|Default|SetcurState state))
  (switch string _output_get
    (:开启
      (Variables|Default|SetcurWidget _widget)
      (Transformation|SetWorldScale3D _normal "1.000000,1.000000,1.000000")
      (Transformation|SetWorldScale3D _close "0, 0, 0")
      (Transformation|SetWorldScale3D _warning "0, 0, 0")
      (bind _asbp_ui_temperature_display_normal (Utilities|Casting|CastToBP_UI_TemperatureDisplay_Normal (UserInterface|GetUserWidgetObject _widget)))
      (Default|InitTemperature _asbp_ui_temperature_display_normal (Variables|Default|Gettemperature)))
    (:关闭
      (Variables|Default|SetcurWidget (Variables|Default|GetWidget1))
      (Transformation|SetWorldScale3D _normal "0, 0, 0")
      (Transformation|SetWorldScale3D _close "1.000000,1.000000,1.000000")
      (Transformation|SetWorldScale3D _warning "0, 0, 0"))
    (:警告
      (Variables|Default|SetcurWidget (Variables|Default|GetWidget2))
      (Transformation|SetWorldScale3D _normal "0, 0, 0")
      (Transformation|SetWorldScale3D _close "0, 0, 0")
      (Transformation|SetWorldScale3D _warning "1.000000,1.000000,1.000000"))))

(event EventBeginPlay
  (Input|EnableInput (Game|GetPlayerController 0))
  (Variables|Default|Setid (.RightS (Utilities|String|Split (Utilities|GetDisplayName self) "BP_IOT_Air_Conditioner")))
  (Variables|Default|SetcurWidget (Variables|Default|GetWidget2))
  (bind _returnvalue (Actor|GetActorOfClass "/Game/Common/Blueprints/Sence/DC/DCLogic.DCLogic_C"))
  (Variables|Default|SetdcLogic _returnvalue))

(event EventTick
  (params (DeltaSeconds :type Float%20%28single-precision%29))
  (Utilities|FlowControl|Sequence
    (:then_0
      ;[1 1 1] 标签跟随镜头
      (Transformation|SetWorldRotation (Variables|Default|GetcurWidget) (Math|Rotator|FindLookatRotation (Transformation|GetActorLocation self) (Transformation|GetActorLocation (Game|GetPlayerCameraManager 0))) false false))
    (:then_1
      ;[1 1 1] 扇叶旋转
      (if (Utilities|Enum|Equal(Enum) (Variables|Default|GetcurState) "开启")
        (Transformation|AddLocalRotation (Variables|Default|GetSM_FSYZ) "0,10.000000, 0" false false)))))

(fn ConstructionScript)

(fn InitItem
  (params (id :type String) (state :type String) (remarks :type Boolean) (temperature :type String) (operateState :type Boolean))
  (Variables|Default|Setid id)
  (Variables|Default|SetcurState state)
  (Variables|Default|Settemperature temperature)
  (Variables|Default|Setremarks remarks)
  (Variables|Default|SetoperateState operateState)
  (CallFunction|InitAirCondition state))

(fn SetTemperature
  (params (temperature :type String)))