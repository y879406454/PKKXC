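; Clickable IoT monitoring camera marker that shows a normal or abnormal state and opens the matching camera dialog.
; initCamera toggles the Normal and Warming components by scale, while BeginPlay derives the Id from the actor's display name.
; Widget and mesh clicks create web-based viewports, whose interface events close the dialogs or open a MediaPanel.
; Tick turns the first widget toward the player camera.
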(event OnClicked(Widget)
  (params (TouchedComponent :type Primitive%20Component%20Object%20Reference) (ButtonPressed :type Key%20Structure :default "None"))
  (bind _returnvalue (UserInterface|CreateWidget "/Game/Common/Blueprints/IOT/Monitor/Cameras_Viewport.Cameras_Viewport_C"))
  (UserInterface|Viewport|AddtoViewport _returnvalue 0)
  (EventDispatchers|BindEventtoOnInterfaceEvent (Variables|/Game/Common/Blueprints/IOT/Monitor/Cameras_Viewport.Cameras_Viewport_C|GetWebInterface_35 _returnvalue) (delegate Custom|onBroadcast)))

(event OnClicked(StaticMesh)
  (params (TouchedComponent :type Primitive%20Component%20Object%20Reference) (ButtonPressed :type Key%20Structure :default "None"))
  (bind _returnvalue (UserInterface|CreateWidget "/Game/Common/Blueprints/IOT/Monitor/Cameras_Viewport.Cameras_Viewport_C"))
  (UserInterface|Viewport|AddtoViewport _returnvalue 0)
  (EventDispatchers|BindEventtoOnInterfaceEvent (Variables|/Game/Common/Blueprints/IOT/Monitor/Cameras_Viewport.Cameras_Viewport_C|GetWebInterface_35 _returnvalue) (delegate Custom|onBroadcast)))

(event OnClicked(Widget1)
  (params (TouchedComponent :type Primitive%20Component%20Object%20Reference) (ButtonPressed :type Key%20Structure :default "None"))
  (bind _returnvalue (UserInterface|CreateWidget "/Game/Common/Blueprints/IOT/Monitor/Cameras_error_Viewport.Cameras_error_Viewport_C"))
  (UserInterface|Viewport|AddtoViewport _returnvalue 0)
  (EventDispatchers|BindEventtoOnInterfaceEvent (Variables|/Game/Common/Blueprints/IOT/Monitor/Cameras_error_Viewport.Cameras_error_Viewport_C|GetWebInterface_35 _returnvalue) (delegate Custom|onBroadcast)))

(event OnClicked(StaticMesh1)
  (params (TouchedComponent :type Primitive%20Component%20Object%20Reference) (ButtonPressed :type Key%20Structure :default "None"))
  (bind _returnvalue (UserInterface|CreateWidget "/Game/Common/Blueprints/IOT/Monitor/Cameras_error_Viewport.Cameras_error_Viewport_C"))
  (UserInterface|Viewport|AddtoViewport _returnvalue 0)
  (EventDispatchers|BindEventtoOnInterfaceEvent (Variables|/Game/Common/Blueprints/IOT/Monitor/Cameras_error_Viewport.Cameras_error_Viewport_C|GetWebInterface_35 _returnvalue) (delegate Custom|onBroadcast)))

(event Custom|onBroadcast
  (params (Name :type Name) (Data :type Json%20Library%20Value%20Structure) (Callback :type Web%20Interface%20Callback%20Structure))
  (switch name Name
    (:closeCameraDialog
      (Widget|RemovefromParent (stale OnClicked(Widget) _returnvalue)))
    (:closeCameraDialogError
      (Widget|RemovefromParent (stale OnClicked(Widget1) _returnvalue)))
    (:openWindow
      (bind _returnvalue (UserInterface|CreateWidget "/Game/Common/Blueprints/IOT/Monitor/MediaPanel.MediaPanel_C"))
      (UserInterface|Viewport|AddtoViewport _returnvalue 0))))

(event Custom|initCamera
  (params (state :type String))
  (bind _normal (Variables|Default|GetNormal))
  (bind _warming (Variables|Default|GetWarming))
  (switch string state
    (:正常
      (Transformation|SetWorldScale3D _normal "1.000000,1.000000,1.000000")
      (Transformation|SetWorldScale3D _warming "0, 0, 0"))
    (:异常
      (Transformation|SetWorldScale3D _normal "0, 0, 0")
      (Transformation|SetWorldScale3D _warming "1.000000,1.000000,1.000000"))))

(event EventBeginPlay
  (Variables|Default|Setid (.RightS (Utilities|String|Split (Utilities|GetDisplayName self) "Cameras_Controller_BP"))))

(event EventTick
  (params (DeltaSeconds :type Float%20%28single-precision%29))
  (Transformation|SetWorldRotation (Variables|Default|GetWidget) (Math|Rotator|FindLookatRotation (Transformation|GetActorLocation self) (Transformation|GetActorLocation (Game|GetPlayerCameraManager 0))) false false))

(fn ConstructionScript)