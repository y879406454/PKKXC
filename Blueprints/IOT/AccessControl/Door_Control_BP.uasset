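; Clickable door access-control marker actor for an IoT scene.
; Clicking its mesh or widget calls 展示门禁信息 (show access-control info) on MyController.
; Every tick, the widget rotates to face the player camera and scales up while Controller.IsGod is true, collapsing to zero otherwise.
; BeginPlay runs GetActorOfClass lookups but sets both controller references to None.
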(event OnClicked(Widget)
  (params (TouchedComponent :type Primitive%20Component%20Object%20Reference) (ButtonPressed :type Key%20Structure :default "None"))
  (CallFunction|展示门禁信息 (.myController (Variables|Default|GetmyController))))

(event OnClicked(StaticMeshComponent)
  (params (TouchedComponent :type Primitive%20Component%20Object%20Reference) (ButtonPressed :type Key%20Structure :default "None"))
  (CallFunction|展示门禁信息 (.myController (Variables|Default|GetmyController))))

(event EventTick
  (params (DeltaSeconds :type Float%20%28single-precision%29))
  (Transformation|SetWorldRotation (Variables|组件|GetWidget) (Math|Rotator|FindLookatRotation (Transformation|GetActorLocation self) (Transformation|GetActorLocation (Game|GetPlayerCameraManager 0))) false false)
  (if (Variables|Default|GetIsGod (.controller (Variables|Default|Getcontroller)))
    (Transformation|SetWorldScale3D (Variables|组件|GetWidget) "2.000000,2.000000,2.000000")
    (else
      (Transformation|SetWorldScale3D (Variables|组件|GetWidget) "0, 0, 0"))))

(event EventBeginPlay
  (bind _returnvalue (Actor|GetActorOfClass 0))
  (Variables|Default|SetmyController 0 _returnvalue)
  (bind _returnvalue_2 (Actor|GetActorOfClass 0))
  (Variables|Default|Setcontroller 0 _returnvalue_2))

(fn ConstructionScript)